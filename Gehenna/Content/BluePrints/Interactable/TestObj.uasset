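; TestObj is a test interactable that turns player input into interaction calls.
; Pressing Fire calls StartInteraction.
; Each Tick polls the MoveRight and MoveForward axes and passes one direction to ReceiveInput while an axis is past a threshold, checking horizontal before vertical.
; It has no edge detection, so a held direction repeats every frame; a debug axis print is left unconnected.
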(event EventBeginPlay)

(event Collision|EventActorBeginOverlap
  (params (OtherActor :type Actor%20Object%20Reference)))

(event EventTick
  (params (DeltaSeconds :type Float%20%28single-precision%29))
  (bind _returnvalue (Input|AxisValues|GetMoveRight))
  (bind _returnvalue_2 (Input|AxisValues|GetMoveForward))
  (if (<= _returnvalue -0.75)
    (Class|InteractableObj|ReceiveInput "VE_Left")
    (elif (>= _returnvalue 0.75)
      (Class|InteractableObj|ReceiveInput "VE_Right")
      (elif (<= _returnvalue_2 -0.75)
        (Class|InteractableObj|ReceiveInput "VE_Down")
        (elif (>= _returnvalue_2 0.75)
          (Class|InteractableObj|ReceiveInput "VE_Up"))))))

(event Input|ActionEvents|InputActionFire
  (params (Key :type Key%20Structure))
  (:Pressed
    (Class|InteractableObj|StartInteraction)))

(fn ConstructionScript)