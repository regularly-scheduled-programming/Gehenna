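; Prototype test character for AI sight perception that shows whether it senses the player.
; On BeginPlay it registers the player controller as a sight stimuli source and sets its state text to idle.
; Each perception update reads the player pawn's first last-sensed stimulus from AIPerception, then switches the text between attacking and idle and prints the state, with no actual attack logic.
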(event OnPerceptionUpdated(AIPerception)
  (params (UpdatedActors :type Array%20of%20Actor%20Object%20References))
  ;[0.8177 0.1656 0.4252] Prototype Sight Perception Tracking With AIPerception Component
  (bind _info (Class|AIPerceptionComponent|GetActorsPerception (Variables|Default|GetAIPerception) (Game|Player|GetPlayerPawn 0)))
  (if (.bSuccessfullySensed (Utilities|Struct|BreakAIStimulus (Utilities|Array|Get(acopy) (.LastSensedStimuli (Utilities|Struct|BreakActorPerceptionBlueprintInfo _info)))))
    (Development|PrintString "Attack")
    (Rendering|Components|TextRender|SetText (Variables|Default|GetStateText) (Variables|Default|GetAttackingDebugString))
    (else
      (Development|PrintString "Idle")
      (Rendering|Components|TextRender|SetText (Variables|Default|GetStateText) (Variables|Default|GetIdleDebugString)))))

(event EventBeginPlay
  ;[0.2026 1 0.2461] Register Targets To Sense
  (Class|AIPerceptionSystem|RegisterPerceptionStimuliSource "/Script/AIModule.AISense_Sight" (Game|GetPlayerController 0))
  (Rendering|Components|TextRender|SetText (Variables|Default|GetStateText) (Variables|Default|GetIdleDebugString)))

(fn ConstructionScript)